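; Small walker enemy pawn that spawns its default controller and attacks Player-tagged actors with a laser and an expanding EMP cylinder.
; Point damage lowers overall and per-bone health: broken feet enable capsule physics, while zero health or a broken laser socket outside laser mode destroys it.
; Back Foot R drains laser socket health.
; Attack, charge, wall-detection and fall-check functions are exposed without callers here; wall traces set a surface-aligned rotation.
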(event `self.ReceiveBeginPlay`
  (`self.SpawnDefaultController`))

(event `self.ReceiveTick`
  (params (DeltaSeconds :type "Float (single-precision)")))

(event `self.Cylinder.OnComponentBeginOverlap`
  (params (OverlappedComponent :type "PrimitiveComponent Object Reference") (OtherActor :type "Actor Object Reference") (OtherComp :type "PrimitiveComponent Object Reference") (OtherBodyIndex :type Integer) (bFromSweep :type Boolean) (SweepResult :type "HitResult Structure (by ref)"))
  (if (`self.ActorHasTag` OtherActor "Player")
    (`GameplayStatics.ApplyPointDamage` OtherActor 5.0 (`self.K2_GetActorLocation`) SweepResult null self)))

(event `self.ReceivePointDamage`
  (params (Damage :type "Float (single-precision)") (DamageType :type "DamageType Object Reference") (HitLocation :type "Vector Structure") (HitNormal :type "Vector Structure") (HitComponent :type "PrimitiveComponent Object Reference") (BoneName :type Name) (ShotFromDirection :type "Vector Structure") (InstigatedBy :type "Controller Object Reference") (DamageCauser :type "Actor Object Reference") (HitInfo :type "HitResult Structure (by ref)"))
  ;[0 1 0.1535] 体力管理
  (`KismetSystemLibrary.PrintString` (`KismetStringLibrary.Conv_NameToString` BoneName))
  (set `self.Health` (- (`self.Health`) Damage))
  (`self.PartsDamage` BoneName Damage)
  (if (<= (`self.Health`) 0.0)
    (`/Engine/EditorBlueprintResources/StandardMacros.DoOnce` false
      (:`Completed`
        (`self.Death`)))))

(event `self.ReceiveRadialDamage`
  (params (DamageReceived :type "Float (single-precision)") (DamageType :type "DamageType Object Reference") (Origin :type "Vector Structure") (HitInfo :type "HitResult Structure (by ref)") (InstigatedBy :type "Controller Object Reference") (DamageCauser :type "Actor Object Reference"))
  ;[0 1 0.1535] 体力管理
  (set `self.Health` (- (`self.Health`) 1.0))
  (if (<= (`self.Health`) 0.0)
    (`/Engine/EditorBlueprintResources/StandardMacros.DoOnce` false
      (:`Completed`
        (`self.Death`)))))

(event `PartsDamage`
  (params (NewParam :type Name) (NewParam2 :type "Float (double-precision)"))
  ;[0 1 0.1535] 体力管理
  (switch `name` NewParam
    (:`FrontFoot_R`
      (bind _output_get (set `self.FrontLegRHealth` (- (`self.FrontLegRHealth`) NewParam2)))
      (if (<= _output_get 0.0)
        (`/Engine/EditorBlueprintResources/StandardMacros.DoOnce` false
          (:`Completed`
            (`PrimitiveComponent.SetSimulatePhysics` (`self.CapsuleComponent`) true :!label _label)))))
    (:`FrontFoot_L`
      (bind _output_get_2 (set `self.FrontLegLHealth` (- (`self.FrontLegLHealth`) NewParam2)))
      (if (<= _output_get_2 0.0)
        (`/Engine/EditorBlueprintResources/StandardMacros.DoOnce` false
          (:`Completed`
            (goto _label)))))
    (:`BackFoot_L`
      (bind _output_get_3 (set `self.BackLegRHealth` (- (`self.BackLegRHealth`) NewParam2)))
      (if (<= _output_get_3 0.0)
        (`/Engine/EditorBlueprintResources/StandardMacros.DoOnce` false
          (:`Completed`
            (goto _label)))))
    (:`BackFoot_R`
      (bind _output_get_4 (set `self.LaserSocketHealth` (- (`self.LaserSocketHealth`) NewParam2)))
      (if (<= _output_get_4 0.0)
        (`/Engine/EditorBlueprintResources/StandardMacros.DoOnce` false
          (:`Completed`
            (goto _label)))))
    (:`laserSocket`
      (if (not (`self.IsLaserMode`))
        (bind _output_get_5 (set `self.LaserSocketHealth` (- (`self.LaserSocketHealth`) NewParam2)))
        (if (<= _output_get_5 0.0)
          (`/Engine/EditorBlueprintResources/StandardMacros.DoOnce` false
            (:`Completed`
              (`self.Death`))))))))

(fn `BurstEMP`
  (returns (End :type Boolean))
  (bind _cylinder (`self.Cylinder`))
  (bind _cylinder_2 (`self.Cylinder`))
  (set `self.BurstBool` true)
  (bind _output_get (set `self.EMPRadius` (+ (`self.EMPRadius`) (`self.RadiusSpreadSpeed`))))
  (`SceneComponent.SetVisibility` _cylinder_2 true false)
  (`SceneComponent.SetRelativeScale3D` _cylinder_2 (`KismetMathLibrary.MakeVector` _output_get _output_get))
  (if (> (`self.EMPRadius`) (`self.MaxRadius`))
    (bind _output_get_2 (set `self.EMPRadius` 0.1))
    (`SceneComponent.SetRelativeScale3D` _cylinder (`KismetMathLibrary.MakeVector` _output_get_2 _output_get_2))
    (`SceneComponent.SetVisibility` _cylinder false false)
    (return true)
    (else
      (return false))))

(fn `BurstLaser`
  (bind (_returnvalue_location _returnvalue_rotation) (`KismetMathLibrary.BreakTransform` (`SceneComponent.GetSocketTransform` (`self.Mesh`) "LaserMuzzleSoc" "RTS_World")))
  (bind _returnvalue (* (`KismetMathLibrary.GetForwardVector` _returnvalue_rotation) (`self.LaserLength`)))
  (set `self.BurstBool` true)
  ;[1 1 1] t
  (bind _outhit (`KismetSystemLibrary.LineTraceSingle` :`Start` _returnvalue_location :`End` _returnvalue :`TraceChannel` "TraceTypeQuery3" :`DrawDebugType` "ForOneFrame"))
  (bind (_bblockinghit _binitialoverlap _time _distance _location _impactpoint _normal _impactnormal _physmat _hitactor) (`GameplayStatics.BreakHitResult` _outhit))
  (if (`KismetSystemLibrary.IsValid` _hitactor)
    (if (`self.ActorHasTag` _hitactor "Player")
      (`GameplayStatics.ApplyPointDamage` _hitactor 10.0 _returnvalue_location _outhit null self)))
  (bind _returnvalue_2 (`GameplayStatics.SpawnEmitterAtLocation` "/Game/VRWireContents/Effects/Beam/P_Beam.P_Beam" _returnvalue_location))
  (`FXSystemComponent.SetVectorParameter` _returnvalue_2 "None" (- _returnvalue _returnvalue_location)))

(fn `Charge`
  (set `self.ChargeBool` true))

(fn `Death`
  (`self.K2_DestroyActor`))

(fn `Detect Wall`
  (returns (Hit :type Boolean))
  (bind _returnvalue (`self.GetActorForwardVector`))
  (bind _returnvalue_2 (+ (`self.K2_GetActorLocation`) (0.0 0.0 0.0)))
  (`|ExecutionSequence`
    (:`then_0`
      ;[1 1 1] 前方の壁
      (bind (_outhit _returnvalue_3) (`KismetSystemLibrary.LineTraceSingle` :`Start` _returnvalue_2 :`End` (+ _returnvalue_2 (* _returnvalue 500.0)) :`TraceChannel` "TraceTypeQuery3" :`DrawDebugType` "ForOneFrame" :`TraceColor` (struct :`G` 0.080823 :`B` 1.0 :`A` 1.0)))
      (if _returnvalue_3
        (set `self.RotateValue` (`KismetMathLibrary.MakeRotFromZX` (`.Normal` (`GameplayStatics.BreakHitResult` _outhit)) _returnvalue))
        (return true)))))

(fn `IsFall`
  (bind (_outhit _returnvalue) (`KismetSystemLibrary.LineTraceSingle` (`self.K2_GetActorLocation`) (* (`self.GetActorUpVector`) -30.0) "TraceTypeQuery3"))
  (if _returnvalue
    (set `self.IsFalling` false)
    (else
      (set `self.IsFalling` true))))

(fn `UserConstructionScript`)