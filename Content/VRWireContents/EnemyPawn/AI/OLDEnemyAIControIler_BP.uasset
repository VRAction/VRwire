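; AI controller for EnemyPawn that runs its behavior tree with patrol and cover points taken from the pawn.
; AI perception records sight and hearing of tagged actors, reading stimuli by fixed index.
; Tick raises a clamped, decaying warning level by inverse-square player distance while seen.
; Helper functions add hearing-based warning, serve patrol/cover locations, or max the warning with a sound and player-instigated noise at the enemy.
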(event `self.ReceiveBeginPlay`
  (bind _asenemy_pawn (cast `/Game/VRWireContents/EnemyPawn/EnemyPawn` (`self.K2_GetPawn`)))
  (set `self.AI_PatrolPoints` (`/Game/VRWireContents/EnemyPawn/EnemyPawn.PatrolPoints` _asenemy_pawn))
  (set `self.AI_CoverPoints` (`/Game/VRWireContents/EnemyPawn/EnemyPawn.CoverPoint` _asenemy_pawn))
  (`self.UseBlackboard` "/Game/VRWireContents/EnemyPawn/AI/Enemy_BB.Enemy_BB")
  (`BlackboardComponent.SetValueAsFloat` (`AIBlueprintHelperLibrary.GetBlackboard` null) "PatrolWaitDuration" (`/Game/VRWireContents/EnemyPawn/EnemyPawn.PatrolWaitDuration` _asenemy_pawn))
  (`self.RunBehaviorTree` "/Game/VRWireContents/EnemyPawn/AI/EnemyAI_BT.EnemyAI_BT"))

(event `self.ReceiveTick`
  (params (DeltaSeconds :type "Float (single-precision)"))
  (`|ExecutionSequence`
    (:`then_0`
      (if (`self.SeePlayer`)
        (`self.Add WPBy Seen`)))
    (:`then_1`
      (`self.Calc WP` DeltaSeconds))))

(event `self.AIPerception.OnPerceptionUpdated`
  (params (UpdatedActors :type "Array of Actor Object Reference (by ref)"))
  (for _array_element UpdatedActors
    (if (`self.ActorHasTag` _array_element (`self.WatchTag`))
      (bind _info (`AIPerceptionComponent.GetActorsPerception` (`self.AIPerception`) _array_element))
      (`|ExecutionSequence`
        (:`then_0`
          (bind (_target _lastsensedstimuli) (break `ActorPerceptionBlueprintInfo` _info))
          (bind (_age _expirationage _strength _stimuluslocation _receiverlocation _tag _bsuccessfullysensed) (break `AIStimulus` (`|GetArrayItem` _lastsensedstimuli)))
          (bind _output_get (set `self.SeePlayer` _bsuccessfullysensed))
          (if (not _output_get)
            (set `self.PlayerSeenPosition` _stimuluslocation)
            (set `self.MySeenPosition` _receiverlocation)))
        (:`then_1`
          (bind (_age_2 _expirationage_2 _strength_2 _stimuluslocation_2 _receiverlocation_2 _tag_2 _bsuccessfullysensed_2) (break `AIStimulus` (`|GetArrayItem` _lastsensedstimuli 1)))
          (bind _output_get_2 (set `self.HearPlayer` _bsuccessfullysensed_2))
          (if _output_get_2
            (set `self.PlayerHearPosition` _stimuluslocation_2)
            (set `self.MyHearPosition` _receiverlocation_2)
            (set `self.HearStrength` _strength_2)))))))

(fn `Add WPBy Hear`
  (set `self.WarningPoint` (+ (`self.WarningPoint`) (* (`self.HearStrength`) 80.0))))

(fn `Add WPBy Seen`
  (set `self.WarningPoint` (+ (`self.WarningPoint`) (* (/ 100000.0 (`KismetMathLibrary.Square` (`KismetMathLibrary.Vector_Distance` (`self.K2_GetActorLocation` (`GameplayStatics.GetPlayerCharacter` 0)) (`self.K2_GetActorLocation`)))) 50.0))))

(fn `Calc WP`
  (params (DeltaTime :type "Float (double-precision)"))
  (`|ExecutionSequence`
    (:`then_0`
      (set `self.WarningPoint` (- (`self.WarningPoint`) (* DeltaTime (`self.SubtructWP`)))))
    (:`then_1`
      (if (> (`self.WarningPoint`) 150.0)
        (set `self.WarningPoint` 150.0)))
    (:`then_2`
      (if (< (`self.WarningPoint`) 0.0)
        (bind _output_get (set `self.WarningPoint` 0.0))))))

(fn `GetCoverLocation`
  (returns (CoverPoint :type "Vector Structure"))
  (bind _output (`|GetArrayItem` (`self.AI_CoverPoints`) (`self.CoverIndex`)))
  (if (`KismetSystemLibrary.IsValid` _output)
    (return (`self.K2_GetActorLocation` _output))))

(fn `GetPatrolLocation`
  (returns (ReturnValue :type "Vector Structure"))
  (bind _output (`|GetArrayItem` (`self.AI_PatrolPoints`) (`self.PatrolIndex`)))
  (if (`KismetSystemLibrary.IsValid` _output)
    (return (`self.K2_GetActorLocation` _output))))

(fn `OnRep_WatchTag`)

(fn `POPPatrolLocation`
  (bind _output_get (set `self.PatrolIndex` (mod (+ (`self.PatrolIndex`) 1) (`KismetArrayLibrary.Array_Length` (`self.AI_PatrolPoints`))))))

(fn `UserConstructionScript`)

(fn `WPMax`
  (bind _returnvalue (`self.K2_GetActorLocation` (cast `/Game/VRWireContents/EnemyPawn/EnemyPawn` (`self.K2_GetPawn`) :!pure true)))
  (set `self.WarningPoint` 150.0)
  (`GameplayStatics.PlaySoundAtLocation` "/Game/VRWireContents/Sounds/EnemySounds/SC_EnemyDetected.SC_EnemyDetected" _returnvalue (struct) 1.0 1.0 0.0 null null null)
  (`self.MakeNoise` 1.0 (`GameplayStatics.GetPlayerPawn` 0) _returnvalue 6000.0))