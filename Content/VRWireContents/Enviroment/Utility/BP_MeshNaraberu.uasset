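; BP_MeshNaraberu is an environment utility actor that tiles a chosen static mesh in a grid.
; Its construction script loops over vertical and horizontal counts, adding a mesh component per cell, spaced by the mesh's bounds.
; TillingAxis selects the plane: X lays tiles in XY with Offset added, while Z stacks them in YZ without it.
; The event graph has no active logic.
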(fn `UserConstructionScript`
  (bind _returnvalue (`StaticMesh.GetBounds` (`self.StaticMesh`)))
  (bind _returnvalue_2 (* (.y (`.BoxExtent` (`KismetMathLibrary.BreakBoxSphereBounds` _returnvalue))) 2.0))
  (for _index (range (+ (`self.VetricalNum`) 1))
    (for _index_2 (range (+ (`self.HorizontalNum`) 1))
      (switch `EPlaneConstraintAxisSetting` (`self.TillingAxis`)
        (:`X`
          (bind _returnvalue_3 (`AddComponent|NODE_AddStaticMeshComponent-2` :`RelativeTransform` (`KismetMathLibrary.MakeTransform` (+ (`KismetMathLibrary.MakeVector` (* _index_2 (* (.x (`.BoxExtent` (`KismetMathLibrary.BreakBoxSphereBounds` _returnvalue))) 2.0)) (* _index _returnvalue_2)) (`self.offset`)))))
          (`StaticMeshComponent.SetStaticMesh` _returnvalue_3 (`self.StaticMesh`)))
        (:`Z`
          (bind _returnvalue_4 (`AddComponent|NODE_AddStaticMeshComponent-0` :`RelativeTransform` (`KismetMathLibrary.MakeTransform` (`KismetMathLibrary.MakeVector` 0.0 (* _index_2 _returnvalue_2) (* _index (* (.z (`.BoxExtent` (`KismetMathLibrary.BreakBoxSphereBounds` _returnvalue))) 2.0))))))
          (`StaticMeshComponent.SetStaticMesh` _returnvalue_4 (`self.StaticMesh`)))))))