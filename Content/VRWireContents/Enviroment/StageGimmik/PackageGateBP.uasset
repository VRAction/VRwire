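; PackageGateBP is a stage gimmick gate that checks whether the player carries a required inventory item.
; When a Player-tagged RobotJOE enters the box, it looks up the gate's Name in that player's Inventory.
; If found, it hides the mesh after a short delay and plays a sound; otherwise it launches and teleports the player downward and applies damage.
; DebugMode skips the whole check.
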(event `self.Box.OnComponentBeginOverlap`
  (params (OverlappedComponent :type "PrimitiveComponent Object Reference") (OtherActor :type "Actor Object Reference") (OtherComp :type "PrimitiveComponent Object Reference") (OtherBodyIndex :type Integer) (bFromSweep :type Boolean) (SweepResult :type "HitResult Structure (by ref)"))
  (bind _asrobot_joe (cast `/Game/VRWireContents/JOEBlueprint/RobotJOE` OtherActor :!pure true))
  (if (`self.DebugMode`)
    _
    (elif (`KismetSystemLibrary.IsValid` OtherActor)
      (if (`self.ActorHasTag` OtherActor "Player")
        (if (`.ReturnValue` (`BlueprintMapLibrary.Map_Find` (`/Game/VRWireContents/JOEBlueprint/RobotJOE.Inventory` _asrobot_joe) (`self.Name`)))
          (`KismetSystemLibrary.Delay` 0.5)
          (`SceneComponent.SetVisibility` (`self.StaticMeshComponent`) false false)
          (`GameplayStatics.PlaySound2D` "/Game/VRWireContents/Sounds/SoundResources/SoundStraipe/UI/Click_Positive_Medium_02.Click_Positive_Medium_02" 1.0 1.0 0.0 null null)
          (else
            (`Character.LaunchCharacter` _asrobot_joe (0.0 0.0 -1000.0) false true)
            (`self.K2_SetActorLocation` _asrobot_joe (+ (`self.K2_GetActorLocation` _asrobot_joe) (0.0 0.0 -100.0)) false true)
            (`GameplayStatics.ApplyDamage` _asrobot_joe 1.0 null self)))))))

(fn `UserConstructionScript`)