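; Rotating electric blade stage gimmick that damages and knocks back the player on contact.
; On BeginPlay it sets the RotatingMovement component's rate from Speed and starts its audio.
; When the Box overlaps an actor tagged Player, it applies fixed damage.
; If that actor is RobotJOE, it also launches the character along the blade actor's up vector, overriding horizontal velocity, and plays an electric damage sound.
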(event `self.ReceiveBeginPlay`
  (set `RotatingMovementComponent.RotationRate` (`KismetMathLibrary.MakeRotator` 0.0 0.0 (`self.Speed`)) (`self.RotatingMovement`))
  (`AudioComponent.Play` (`self.Audio`) 0.0))

(event `self.Box.OnComponentBeginOverlap`
  (params (OverlappedComponent :type "PrimitiveComponent Object Reference") (OtherActor :type "Actor Object Reference") (OtherComp :type "PrimitiveComponent Object Reference") (OtherBodyIndex :type Integer) (bFromSweep :type Boolean) (SweepResult :type "HitResult Structure (by ref)"))
  (if (`self.ActorHasTag` OtherActor "Player")
    (`GameplayStatics.ApplyDamage` OtherActor 5.0 null self)
    (bind _asrobot_joe (cast `/Game/VRWireContents/JOEBlueprint/RobotJOE` OtherActor))
    (`Character.LaunchCharacter` _asrobot_joe (* (`self.GetActorUpVector`) 1000.0) true false)
    (`GameplayStatics.PlaySound2D` "/Game/VRWireContents/Sounds/EnviromentSounds/ElectricDamage.ElectricDamage" 1.0 1.0 0.0 null null)))

(fn `UserConstructionScript`)