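; RainTriggerBP is a stage gimmick trigger that starts or stops rain when the player enters its collision component.
; On overlap by a "Player"-tagged RobotJOE, the RainStop flag selects between calling the robot's Rain or ClearWeathr function.
; Starting rain fades in the MidRain audio and plays Thunder after a delay, while stopping fades MidRain out.
; Both sounds are silenced on BeginPlay.
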(event `self.ReceiveBeginPlay`
  (`AudioComponent.StopDelayed` (`self.MidRain`) 0.0)
  (`AudioComponent.Stop` (`self.Thunder`)))

(event `self.CollisionComponent.OnComponentBeginOverlap`
  (params (OverlappedComponent :type "PrimitiveComponent Object Reference") (OtherActor :type "Actor Object Reference") (OtherComp :type "PrimitiveComponent Object Reference") (OtherBodyIndex :type Integer) (bFromSweep :type Boolean) (SweepResult :type "HitResult Structure (by ref)"))
  (bind _midrain (`self.MidRain`))
  (if (`self.ActorHasTag` OtherActor "Player")
    (bind _asrobot_joe (cast `/Game/VRWireContents/JOEBlueprint/RobotJOE` OtherActor))
    (if (`self.RainStop`)
      (`/Game/VRWireContents/JOEBlueprint/RobotJOE.ClearWeathr` _asrobot_joe)
      (`AudioComponent.FadeOut` _midrain 0.5 0.0 "Linear")
      (else
        (`/Game/VRWireContents/JOEBlueprint/RobotJOE.Rain` _asrobot_joe)
        (`AudioComponent.FadeIn` _midrain 3.0 1.0 0.0 "Linear")
        (`KismetSystemLibrary.Delay` 4.0)
        (`AudioComponent.Play` (`self.Thunder`) 0.0)))))

(fn `UserConstructionScript`)